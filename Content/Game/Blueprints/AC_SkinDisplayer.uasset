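; Actor component that shows a player's equipped shop skin as a color tint on the owning character's skeletal mesh.
; On BeginPlay the local player queries the account subsystem for the equipped item, then reads its color from the DT_ShopItems icon tint.
; It applies the tint through dynamic materials on the first two slots and, on clients, sends it to the server.
; The SkinColor OnRep applies it on non-local copies.
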(event Custom|OnAccountInfo
  (params (Result :type Boolean) (Data :type Account%20Data%20Structure))
  (bind (_id _name _mail _xp _elo _level _money _chestkeys _inventory _equippeditemid) (Utilities|Struct|BreakAccountData Data))
  (for _array_element _inventory
    (if (Utilities|Enum|Equal(Enum) (.Id (Utilities|Struct|BreakOwnedItemData _array_element)) _equippeditemid)
      (CallFunction|GetSkinInfo (.Id (Utilities|Struct|BreakOwnedItemData _array_element))))))

(event Custom|GetSkinInfo
  (params (ItemInstanceID :type String))
  (bind _searchskinitem (Variables|Default|GetSearchSkinItem))
  (Utilities|Array|Clear _searchskinitem)
  (Utilities|Array|Add _searchskinitem ItemInstanceID)
  (Class|AccountSubsystem|GetItemsbyOwnedID (Subsystems|GetAccountSubsystem) (Variables|Default|GetSearchSkinItem) (delegate Custom|OnSkinInfo)))

(event Custom|OnSkinInfo
  (params (Result :type Boolean) (Data :type Array%20of%20Shop%20Item%20Data%20Structures))
  (if Result
    (if (> (Utilities|Array|Length Data) 0)
      (CallFunction|SetSkin (.Name (Utilities|Struct|BreakShopItemData (Utilities|Array|Get(acopy) Data)))))))

(event Custom|Server_SetSkinColor
  (params (Color :type Linear%20Color%20Structure))
  (Variables|Default|SetSkinColor Color))

(event EventBeginPlay
  (bind _returnvalue (CallFunction|IsLocal))
  (if _returnvalue
    (Class|AccountSubsystem|GetAccountInformation (Subsystems|GetAccountSubsystem) (delegate Custom|OnAccountInfo))))

(fn SetSkin
  (params (SkinName :type String))
  (bind _returnvalue (Utilities|GetDataTableRow "/Game/Game/Data/DT_ShopItems.DT_ShopItems" (Utilities|String|StringToName (Utilities|String|Replace SkinName " ")))
    (:then
      (CallFunction|ApplySkinColor (.SpecifiedColor (Utilities|Struct|BreakSlateColor (.TintColor (Utilities|Struct|BreakSlateBrush (.Icon (Utilities|Struct|BreakStruct_ShopItem _returnvalue)))))))
      (bind _output_get (Variables|Default|SetSkinColor (.SpecifiedColor (Utilities|Struct|BreakSlateColor (.TintColor (Utilities|Struct|BreakSlateBrush (.Icon (Utilities|Struct|BreakStruct_ShopItem _returnvalue))))))))
      (if (Networking|IsServer)
        (return)
        (else
          (CallFunction|ServerSetSkinColor _output_get))))))

(fn ApplySkinColor
  (params (Color :type Linear%20Color%20Structure))
  (bind _returnvalue (Components|GetOwner))
  (bind _returnvalue_2 (Actor|GetComponentbyClass _returnvalue "/Script/Engine.SkeletalMeshComponent"))
  (bind _returnvalue_3 (Rendering|Material|CreateDynamicMaterialInstance _returnvalue_2 0 0 "None" :!class /Script/Engine.PrimitiveComponent))
  (Rendering|Material|SetVectorParameterValue _returnvalue_3 "Tint" Color :!class /Script/Engine.MaterialInstanceDynamic)
  (bind _returnvalue_4 (Rendering|Material|CreateDynamicMaterialInstance _returnvalue_2 1 0 "None" :!class /Script/Engine.PrimitiveComponent))
  (Rendering|Material|SetVectorParameterValue _returnvalue_4 "Tint" Color :!class /Script/Engine.MaterialInstanceDynamic))

(fn OnRepSkinColor
  (bind _returnvalue (CallFunction|IsLocal))
  (if (not _returnvalue)
    (CallFunction|ApplySkinColor (Variables|Default|GetSkinColor))))

(fn IsLocal
  (bind _ascharacter (Utilities|Casting|CastToCharacter (Components|GetOwner))
    (:then
      (Utilities|IsValid (Pawn|GetController _ascharacter)
        (:Is%20Valid
          (return (Pawn|IsLocalPlayerController (Pawn|GetController _ascharacter))))
        (:Is%20Not%20Valid
          _)))
    (:CastFailed
      _))
  (return false))