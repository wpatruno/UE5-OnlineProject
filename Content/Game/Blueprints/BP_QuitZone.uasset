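; BP_QuitZone is a trigger actor that returns the game to the main menu when an actor overlaps it.
; A one-shot OnQuit flag ignores later overlaps.
; On the server it sends a close message through the ServerSubsystem and waits a few seconds before loading MainMenu, while clients wait only briefly before leaving.
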(event EventBeginPlay)

(event Collision|EventActorBeginOverlap
  (params (OtherActor :type Actor%20Object%20Reference))
  (if (not (Variables|Default|GetOnQuit))
    (Variables|Default|SetOnQuit true)
    (if (Class|ServerSubsystem|IsServer (Subsystems|GetServerSubsystem))
      (Development|PrintString "Server closing")
      (Class|ServerSubsystem|SendServerClose (Subsystems|GetServerSubsystem))
      (Utilities|FlowControl|Delay 3.0)
      (else
        (Development|PrintString "Leaving server")
        (Utilities|FlowControl|Delay 0.2)))
    (Game|OpenLevel(byObjectReference) "/Game/Game/Maps/MainMenu.MainMenu")))

(fn ConstructionScript)