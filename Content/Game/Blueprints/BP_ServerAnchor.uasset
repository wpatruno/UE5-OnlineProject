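; BP_ServerAnchor is a level actor that reports the server's lifecycle through ServerSubsystem.
; On a server it sends ready one second after BeginPlay and sends close when destroyed, unless the IsClosedSent flag shows close was already sent.
; Pressing X returns to MainMenu; a server first sends close, sets the flag and waits three seconds, while a client leaves after a short delay.
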(event EventBeginPlay
  (bind _returnvalue (Subsystems|GetServerSubsystem))
  (Utilities|FlowControl|Delay 1.0)
  (if (Class|ServerSubsystem|IsServer _returnvalue)
    (Class|ServerSubsystem|SendServerReady _returnvalue)
    (Development|PrintString "ServerOpen")))

(event EventDestroyed
  (if (Class|ServerSubsystem|IsServer (Subsystems|GetServerSubsystem))
    (if (not (Variables|Default|GetIsClosedSent))
      (Class|ServerSubsystem|SendServerClose (Subsystems|GetServerSubsystem))
      (Development|PrintString "ServerClose"))))

(event Input|KeyboardEvents|X
  (params (Key :type Key%20Structure :default "None"))
  (:Pressed
    (if (Class|ServerSubsystem|IsServer (Subsystems|GetServerSubsystem))
      (Development|PrintString "Server closing")
      (Class|ServerSubsystem|SendServerClose (Subsystems|GetServerSubsystem))
      (Variables|Default|SetIsClosedSent true)
      (Utilities|FlowControl|Delay 3.0)
      (else
        (Development|PrintString "Leaving server")
        (Utilities|FlowControl|Delay 0.2)))
    (Game|OpenLevel(byObjectReference) "/Game/Game/Maps/MainMenu.MainMenu")))

(fn ConstructionScript)