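; BP_ServerInfoDisplay is an in-world display of the game server's ID, name, address, state and type.
; Shortly after BeginPlay, the server copies its data from the server subsystem into ServerData, a RepNotify variable.
; OnRep_ServerData passes it to DisplayServerData, which fills the text components.
; State and type integers are converted to enums and shown by name.
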(event EventBeginPlay
  (Utilities|FlowControl|Delay 0.2)
  (if (Networking|IsServer)
    (Variables|Default|SetServerData (Class|ServerSubsystem|GetServerData (Subsystems|GetServerSubsystem)))))

(fn ConstructionScript)

(fn SetState
  (params (InInt :type Integer))
  (bind _output_get (Variables|Default|SetServerState (Utilities|Enum|ByteToEnumEServerState (Math|Conversions|ToByte(Integer) InInt))))
  (Rendering|Components|TextRender|SetText (Variables|Default|GetTR_State) (Utilities|Text|ToText(String) (Utilities|String|EnumtoString _output_get))))

(fn SetType
  (params (InInt :type Integer))
  (bind _output_get (Variables|Default|SetServerType (Utilities|Enum|ByteToEnumEServerType (Math|Conversions|ToByte(Integer) InInt))))
  (Rendering|Components|TextRender|SetText (Variables|Default|GetTR_Type) (Utilities|Text|ToText(String) (Utilities|String|EnumtoString _output_get))))

(fn OnRepServerData
  (CallFunction|DisplayServerData (Variables|Default|GetServerData)))

(fn DisplayServerData
  (params (GameServerData :type Game%20Server%20Data%20Structure%20%28by%20ref%29))
  (bind (_id _servertype _name _address _port _players _creationtime _updatedtime _lastalivetime _state) (Utilities|Struct|BreakGameServerData GameServerData))
  (Utilities|FlowControl|Sequence
    (:then_0
      (Rendering|Components|TextRender|SetText (Variables|Default|GetTR_ID) (Utilities|Text|ToText(String) _id)))
    (:then_1
      (Rendering|Components|TextRender|SetText (Variables|Default|GetTR_Name) (Utilities|Text|ToText(String) _name)))
    (:then_2
      (Rendering|Components|TextRender|SetText (Variables|Default|GetTR_IP) (Utilities|Text|ToText(String) _address)))
    (:then_3
      (CallFunction|SetState _state))
    (:then_4
      (CallFunction|SetType _servertype))))